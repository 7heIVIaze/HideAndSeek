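; Furniture drawer Blueprint with sliding open/close logic that is currently unwired: the interaction event is empty, so none of it runs.
; The orphaned graph traces from the first-person camera to pick the drawer's static mesh component under the crosshair.
; It toggles that mesh along local Y between closed and open limits, playing a sound and lerping through two timelines.
; A CanOpen flag blocks retriggering during movement.
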(event `/Game/Assets/BluePrints/UI/InteractInterface_BP.OnInteraction`
  (params (PlayerCharacter :type "/Game/FirstPerson/Blueprints/BP_FirstPersonCharacter Object Reference")))

(fn `UserConstructionScript`)