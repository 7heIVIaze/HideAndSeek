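; BP_Spawn is a trigger volume that spawns a BP_Reaper when the first-person character leaves it.
; On the Box's end overlap, it checks that an object reference is invalid and that Stop is unset, then spawns the reaper at SpawnPoint.
; It turns off the reaper's collect mode, sets its status and latches Stop so the spawn happens only once.
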(event `self.Box.OnComponentBeginOverlap`
  (params (OverlappedComponent :type "PrimitiveComponent Object Reference") (OtherActor :type "Actor Object Reference") (OtherComp :type "PrimitiveComponent Object Reference") (OtherBodyIndex :type Integer) (bFromSweep :type Boolean) (SweepResult :type "HitResult Structure (by ref)")))

(event `self.Box.OnComponentEndOverlap`
  (params (OverlappedComponent :type "PrimitiveComponent Object Reference") (OtherActor :type "Actor Object Reference") (OtherComp :type "PrimitiveComponent Object Reference") (OtherBodyIndex :type Integer))
  (cast `/Game/FirstPerson/Blueprints/BP_FirstPersonCharacter` OtherActor)
  (if (`KismetSystemLibrary.IsValid` (`self.Object`))
    _
    (elif (not (`self.Stop`))
      (bind _returnvalue (`|SpawnActorFromClass` "/Game/Assets/AI/Reaper/BP_Reaper.BP_Reaper_C" (`KismetMathLibrary.MakeTransform` (`SceneComponent.K2_GetComponentLocation` (`self.SpawnPoint`))) "Undefined" "OverrideRootScale" null null))
      (set `Reaper_cpp.bIsCollectMode` false _returnvalue)
      (`Reaper_cpp.SetCurrentStatus` _returnvalue 4)
      (set `self.Stop` true))))

(fn `UserConstructionScript`)